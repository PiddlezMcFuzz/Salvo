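; Ocean manager that computes Gerstner wave displacement on the CPU and applies buoyancy to physics components.
; On construction and BeginPlay it caches global settings and two eight-wave sets from the MPC_WaveParams material parameter collection.
; GetWaveHeight averages both sets, the second with an angle offset.
; ProcessBuoyancy tests a point against that height, then adds upward or downward force there, scaled by cubed, clamped depth, mass and point count.
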(event `self.ReceiveBeginPlay`
  (`self.Init Global Parameters`)
  (`self.Init Wave Set 1`)
  (`self.Init Wave Set 2`))

(fn `Calculate Gerstner`
  (params (`World Position` :type "Vector Structure") (`Direction V2` :type "Vector Structure") (`World Rotation` :type "Float (double-precision)") (Wavelength :type "Float (double-precision)") (Amplitude :type "Float (double-precision)") (Steepness :type "Float (double-precision)") (Time :type "Float (double-precision)"))
  (returns (Displacement :type "Vector Structure"))
  (bind _returnvalue (`KismetMathLibrary.Normal` (`KismetMathLibrary.RotateAngleAxis` `Direction V2` (`KismetMathLibrary.MapRangeUnclamped` `World Rotation` 0.0 1.0 0.0 360.0))))
  (bind _returnvalue_2 (+ (* (`KismetMathLibrary.Dot_VectorVector` (`KismetMathLibrary.MakeVector` (.x `World Position`) (.y `World Position`)) _returnvalue) (/ (`KismetMathLibrary.MultiplyByPi` 2.0) Wavelength)) Time))
  (bind _returnvalue_3 (* (* (`KismetMathLibrary.Cos` _returnvalue_2) Steepness) Amplitude))
  (return (`KismetMathLibrary.MakeVector` (* (.x _returnvalue) _returnvalue_3) (* (.y _returnvalue) _returnvalue_3) (* (`KismetMathLibrary.Sin` _returnvalue_2) Amplitude))))

(fn `Create Wave Set`
  (params (`World Position` :type "Vector Structure") (`Direction V2` :type "Vector Structure") (`Angle Offset 0-1` :type "Float (double-precision)" :default 0.0) (Time :type "Float (double-precision)") (`Global Wave Parameters` :type "/Game/Salvo/Blueprint/environment/WaveParameters Structure") (`Wave Set Parameters` :type "/Game/Salvo/Blueprint/environment/WaveSet Structure"))
  (returns (Displacement :type "Vector Structure"))
  (bind (_angle _wavelength _amplitude _steepness) (break `/Game/Salvo/Blueprint/environment/WaveParameters` `Global Wave Parameters`))
  (bind (_wave01 _wave02 _wave03 _wave04 _wave05 _wave06 _wave07 _wave08) (break `/Game/Salvo/Blueprint/environment/WaveSet` `Wave Set Parameters`))
  (bind (_angle_2 _wavelength_2 _amplitude_2 _steepness_2) (break `/Game/Salvo/Blueprint/environment/WaveParameters` _wave07))
  (bind (_angle_3 _wavelength_3 _amplitude_3 _steepness_3) (break `/Game/Salvo/Blueprint/environment/WaveParameters` _wave01))
  (bind (_angle_4 _wavelength_4 _amplitude_4 _steepness_4) (break `/Game/Salvo/Blueprint/environment/WaveParameters` _wave08))
  (bind (_angle_5 _wavelength_5 _amplitude_5 _steepness_5) (break `/Game/Salvo/Blueprint/environment/WaveParameters` _wave02))
  (bind (_angle_6 _wavelength_6 _amplitude_6 _steepness_6) (break `/Game/Salvo/Blueprint/environment/WaveParameters` _wave03))
  (bind (_angle_7 _wavelength_7 _amplitude_7 _steepness_7) (break `/Game/Salvo/Blueprint/environment/WaveParameters` _wave04))
  (bind (_angle_8 _wavelength_8 _amplitude_8 _steepness_8) (break `/Game/Salvo/Blueprint/environment/WaveParameters` _wave05))
  (bind (_angle_9 _wavelength_9 _amplitude_9 _steepness_9) (break `/Game/Salvo/Blueprint/environment/WaveParameters` _wave06))
  (bind _returnvalue (+ `Angle Offset 0-1` _angle))
  (return (/ (+ (`self.Calculate Gerstner` `World Position` `Direction V2` (+ _returnvalue _angle_3) (* _wavelength _wavelength_3) (* _amplitude _amplitude_3) (* _steepness _steepness_3) Time) (`self.Calculate Gerstner` `World Position` `Direction V2` (+ _returnvalue _angle_5) (* _wavelength _wavelength_5) (* _amplitude _amplitude_5) (* _steepness _steepness_5) Time) (`self.Calculate Gerstner` `World Position` `Direction V2` (+ _returnvalue _angle_6) (* _wavelength _wavelength_6) (* _amplitude _amplitude_6) (* _steepness _steepness_6) Time) (`self.Calculate Gerstner` `World Position` `Direction V2` (+ _returnvalue _angle_7) (* _wavelength _wavelength_7) (* _amplitude _amplitude_7) (* _steepness _steepness_7) Time) (`self.Calculate Gerstner` `World Position` `Direction V2` (+ _returnvalue _angle_8) (* _wavelength _wavelength_8) (* _amplitude _amplitude_8) (* _steepness _steepness_8) Time) (`self.Calculate Gerstner` `World Position` `Direction V2` (+ _returnvalue _angle_9) (* _wavelength _wavelength_9) (* _amplitude _amplitude_9) (* _steepness _steepness_9) Time) (`self.Calculate Gerstner` `World Position` `Direction V2` (+ _returnvalue _angle_2) (* _wavelength _wavelength_2) (* _amplitude _amplitude_2) (* _steepness _steepness_2) Time) (`self.Calculate Gerstner` `World Position` `Direction V2` (+ _returnvalue _angle_4) (* _wavelength _wavelength_4) (* _amplitude _amplitude_4) (* _steepness _steepness_4) Time)) 8.0)))

(fn `Find Wave Height at Point`
  (params (`Actor Transform` :type "Transform Structure") (`Test Point Location` :type "Vector Structure") (Time :type "Float (double-precision)") (`Test Point Radius` :type "Float (double-precision)"))
  (returns (IsUnderWater :type Boolean) (Amount :type "Float (double-precision)") (Delta :type "Float (double-precision)") (`Wave Intersect Location` :type "Vector Structure") (`Wave Height` :type "Float (double-precision)"))
  (bind _returnvalue (`KismetMathLibrary.TransformLocation` `Actor Transform` `Test Point Location`))
  (bind _z (.z _returnvalue))
  (bind _delta (`self.Get Wave Height` _returnvalue Time))
  (bind _z_2 (.z _delta))
  (bind _returnvalue_2 (- _z_2 _z))
  (return (> _returnvalue_2 0.0) (`KismetMathLibrary.Abs` (`KismetMathLibrary.FClamp` (`KismetMathLibrary.MultiplyMultiply_FloatFloat` (/ _returnvalue_2 `Test Point Radius`) 3.0))) _returnvalue_2 (`KismetMathLibrary.MakeVector` (.x (+ _delta _returnvalue)) (.y (+ _delta _returnvalue)) _z) _z_2))

(fn `Get Wave Height`
  (params (Location :type "Vector Structure") (Time :type "Float (double-precision)"))
  (returns (Delta :type "Vector Structure"))
  (locals (`Sum of Wave` :type "Vector Structure"))
  (bind _wavedirectionv2 (`self.WaveDirectionV2`))
  (bind _global_wave_settings (`self.Global Wave Settings`))
  (bind _displacement (`self.Create Wave Set` Location _wavedirectionv2 0.0 Time _global_wave_settings (`self.WaveSet01`)))
  (bind _displacement_2 (`self.Create Wave Set` Location _wavedirectionv2 (`self.Wave 2 Angle Offset`) Time _global_wave_settings (`self.WaveSet02`)))
  (return (/ (+ _displacement _displacement_2) 2.0)))

(fn `Init Global Parameters`
  (locals (Rotation :type "Float (double-precision)") (Wavelength :type "Float (double-precision)") (Amplitude :type "Float (double-precision)") (Steepness :type "Float (double-precision)") (TimeMultiplier :type "Float (double-precision)"))
  (`|ExecutionSequence`
    (:`then_0`
      (bind _returnvalue (`KismetMaterialLibrary.GetScalarParameterValue` "/Game/Salvo/Assets/Materials/WaveGen/MPC_WaveParams.MPC_WaveParams" "Global Angle"))
      (set `local.Rotation` _returnvalue))
    (:`then_1`
      (bind _returnvalue_2 (`KismetMaterialLibrary.GetScalarParameterValue` "/Game/Salvo/Assets/Materials/WaveGen/MPC_WaveParams.MPC_WaveParams" "Global Wavelength"))
      (set `local.Wavelength` _returnvalue_2))
    (:`then_2`
      (bind _returnvalue_3 (`KismetMaterialLibrary.GetScalarParameterValue` "/Game/Salvo/Assets/Materials/WaveGen/MPC_WaveParams.MPC_WaveParams" "Global Amplitude"))
      (set `local.Amplitude` _returnvalue_3))
    (:`then_3`
      (bind _returnvalue_4 (`KismetMaterialLibrary.GetScalarParameterValue` "/Game/Salvo/Assets/Materials/WaveGen/MPC_WaveParams.MPC_WaveParams" "Global Steepness"))
      (set `local.Steepness` _returnvalue_4))
    (:`then_4`
      (bind _returnvalue_5 (`KismetMaterialLibrary.GetScalarParameterValue` "/Game/Salvo/Assets/Materials/WaveGen/MPC_WaveParams.MPC_WaveParams" "Global Time Multiplier"))
      (set `local.TimeMultiplier` _returnvalue_5))
    (:`then_5`
      (set `self.Global Wave Settings` (make `/Game/Salvo/Blueprint/environment/WaveParameters` (`local.Rotation`) (`local.Wavelength`) (`local.Amplitude`) (`local.Steepness`) (`local.TimeMultiplier`))))
    (:`then_6`
      (bind _returnvalue_6 (`KismetMaterialLibrary.GetVectorParameterValue` "/Game/Salvo/Assets/Materials/WaveGen/MPC_WaveParams.MPC_WaveParams" "Global Direction"))
      (bind (_r _g) (`KismetMathLibrary.BreakColor` _returnvalue_6))
      (set `self.WaveDirectionV2` (`KismetMathLibrary.MakeVector` _r _g)))))

(fn `Init Wave Set 1`
  (`|ExecutionSequence`
    (:`then_0`
      (`|ExecutionSequence`
        (:`then_0`
          (bind _returnvalue (`KismetMaterialLibrary.GetVectorParameterValue` "/Game/Salvo/Assets/Materials/WaveGen/MPC_WaveParams.MPC_WaveParams" "Set01Wave01"))
          (set `self.Set01Wave01` (make `/Game/Salvo/Blueprint/environment/WaveParameters` (break `LinearColor` _returnvalue) (`.G` (break `LinearColor` _returnvalue)) (`.B` (break `LinearColor` _returnvalue)) (`.A` (break `LinearColor` _returnvalue)))))
        (:`then_1`
          (bind _returnvalue_2 (`KismetMaterialLibrary.GetVectorParameterValue` "/Game/Salvo/Assets/Materials/WaveGen/MPC_WaveParams.MPC_WaveParams" "Set01Wave02"))
          (set `self.Set01Wave02` (make `/Game/Salvo/Blueprint/environment/WaveParameters` (break `LinearColor` _returnvalue_2) (`.G` (break `LinearColor` _returnvalue_2)) (`.B` (break `LinearColor` _returnvalue_2)) (`.A` (break `LinearColor` _returnvalue_2)))))
        (:`then_2`
          (bind _returnvalue_3 (`KismetMaterialLibrary.GetVectorParameterValue` "/Game/Salvo/Assets/Materials/WaveGen/MPC_WaveParams.MPC_WaveParams" "Set01Wave03"))
          (set `self.Set01Wave03` (make `/Game/Salvo/Blueprint/environment/WaveParameters` (break `LinearColor` _returnvalue_3) (`.G` (break `LinearColor` _returnvalue_3)) (`.B` (break `LinearColor` _returnvalue_3)) (`.A` (break `LinearColor` _returnvalue_3)))))
        (:`then_3`
          (bind _returnvalue_4 (`KismetMaterialLibrary.GetVectorParameterValue` "/Game/Salvo/Assets/Materials/WaveGen/MPC_WaveParams.MPC_WaveParams" "Set01Wave04"))
          (set `self.Set01Wave04` (make `/Game/Salvo/Blueprint/environment/WaveParameters` (break `LinearColor` _returnvalue_4) (`.G` (break `LinearColor` _returnvalue_4)) (`.B` (break `LinearColor` _returnvalue_4)) (`.A` (break `LinearColor` _returnvalue_4)))))
        (:`then_4`
          (bind _returnvalue_5 (`KismetMaterialLibrary.GetVectorParameterValue` "/Game/Salvo/Assets/Materials/WaveGen/MPC_WaveParams.MPC_WaveParams" "Set01Wave05"))
          (set `self.Set01Wave05` (make `/Game/Salvo/Blueprint/environment/WaveParameters` (break `LinearColor` _returnvalue_5) (`.G` (break `LinearColor` _returnvalue_5)) (`.B` (break `LinearColor` _returnvalue_5)) (`.A` (break `LinearColor` _returnvalue_5)))))
        (:`then_5`
          (bind _returnvalue_6 (`KismetMaterialLibrary.GetVectorParameterValue` "/Game/Salvo/Assets/Materials/WaveGen/MPC_WaveParams.MPC_WaveParams" "Set01Wave06"))
          (set `self.Set01Wave06` (make `/Game/Salvo/Blueprint/environment/WaveParameters` (break `LinearColor` _returnvalue_6) (`.G` (break `LinearColor` _returnvalue_6)) (`.B` (break `LinearColor` _returnvalue_6)) (`.A` (break `LinearColor` _returnvalue_6)))))
        (:`then_6`
          (bind _returnvalue_7 (`KismetMaterialLibrary.GetVectorParameterValue` "/Game/Salvo/Assets/Materials/WaveGen/MPC_WaveParams.MPC_WaveParams" "Set01Wave07"))
          (set `self.Set01Wave07` (make `/Game/Salvo/Blueprint/environment/WaveParameters` (break `LinearColor` _returnvalue_7) (`.G` (break `LinearColor` _returnvalue_7)) (`.B` (break `LinearColor` _returnvalue_7)) (`.A` (break `LinearColor` _returnvalue_7)))))
        (:`then_7`
          (bind _returnvalue_8 (`KismetMaterialLibrary.GetVectorParameterValue` "/Game/Salvo/Assets/Materials/WaveGen/MPC_WaveParams.MPC_WaveParams" "Set01Wave08"))
          (set `self.Set01Wave08` (make `/Game/Salvo/Blueprint/environment/WaveParameters` (break `LinearColor` _returnvalue_8) (`.G` (break `LinearColor` _returnvalue_8)) (`.B` (break `LinearColor` _returnvalue_8)) (`.A` (break `LinearColor` _returnvalue_8)))))))
    (:`then_1`
      (set `self.WaveSet01` (make `/Game/Salvo/Blueprint/environment/WaveSet` (`self.Set01Wave01`) (`self.Set01Wave02`) (`self.Set01Wave03`) (`self.Set01Wave04`) (`self.Set01Wave05`) (`self.Set01Wave06`) (`self.Set01Wave07`) (`self.Set01Wave08`))))))

(fn `Init Wave Set 2`
  (`|ExecutionSequence`
    (:`then_0`
      (`|ExecutionSequence`
        (:`then_0`
          (bind _returnvalue (`KismetMaterialLibrary.GetVectorParameterValue` "/Game/Salvo/Assets/Materials/WaveGen/MPC_WaveParams.MPC_WaveParams" "Set02Wave01"))
          (set `self.Set02Wave01` (make `/Game/Salvo/Blueprint/environment/WaveParameters` (break `LinearColor` _returnvalue) (`.G` (break `LinearColor` _returnvalue)) (`.B` (break `LinearColor` _returnvalue)) (`.A` (break `LinearColor` _returnvalue)))))
        (:`then_1`
          (bind _returnvalue_2 (`KismetMaterialLibrary.GetVectorParameterValue` "/Game/Salvo/Assets/Materials/WaveGen/MPC_WaveParams.MPC_WaveParams" "Set02Wave02"))
          (set `self.Set02Wave02` (make `/Game/Salvo/Blueprint/environment/WaveParameters` (break `LinearColor` _returnvalue_2) (`.G` (break `LinearColor` _returnvalue_2)) (`.B` (break `LinearColor` _returnvalue_2)) (`.A` (break `LinearColor` _returnvalue_2)))))
        (:`then_2`
          (bind _returnvalue_3 (`KismetMaterialLibrary.GetVectorParameterValue` "/Game/Salvo/Assets/Materials/WaveGen/MPC_WaveParams.MPC_WaveParams" "Set02Wave03"))
          (set `self.Set02Wave03` (make `/Game/Salvo/Blueprint/environment/WaveParameters` (break `LinearColor` _returnvalue_3) (`.G` (break `LinearColor` _returnvalue_3)) (`.B` (break `LinearColor` _returnvalue_3)) (`.A` (break `LinearColor` _returnvalue_3)))))
        (:`then_3`
          (bind _returnvalue_4 (`KismetMaterialLibrary.GetVectorParameterValue` "/Game/Salvo/Assets/Materials/WaveGen/MPC_WaveParams.MPC_WaveParams" "Set02Wave04"))
          (set `self.Set02Wave04` (make `/Game/Salvo/Blueprint/environment/WaveParameters` (break `LinearColor` _returnvalue_4) (`.G` (break `LinearColor` _returnvalue_4)) (`.B` (break `LinearColor` _returnvalue_4)) (`.A` (break `LinearColor` _returnvalue_4)))))
        (:`then_4`
          (bind _returnvalue_5 (`KismetMaterialLibrary.GetVectorParameterValue` "/Game/Salvo/Assets/Materials/WaveGen/MPC_WaveParams.MPC_WaveParams" "Set02Wave05"))
          (set `self.Set02Wave05` (make `/Game/Salvo/Blueprint/environment/WaveParameters` (break `LinearColor` _returnvalue_5) (`.G` (break `LinearColor` _returnvalue_5)) (`.B` (break `LinearColor` _returnvalue_5)) (`.A` (break `LinearColor` _returnvalue_5)))))
        (:`then_5`
          (bind _returnvalue_6 (`KismetMaterialLibrary.GetVectorParameterValue` "/Game/Salvo/Assets/Materials/WaveGen/MPC_WaveParams.MPC_WaveParams" "Set02Wave06"))
          (set `self.Set02Wave06` (make `/Game/Salvo/Blueprint/environment/WaveParameters` (break `LinearColor` _returnvalue_6) (`.G` (break `LinearColor` _returnvalue_6)) (`.B` (break `LinearColor` _returnvalue_6)) (`.A` (break `LinearColor` _returnvalue_6)))))
        (:`then_6`
          (bind _returnvalue_7 (`KismetMaterialLibrary.GetVectorParameterValue` "/Game/Salvo/Assets/Materials/WaveGen/MPC_WaveParams.MPC_WaveParams" "Set02Wave07"))
          (set `self.Set02Wave07` (make `/Game/Salvo/Blueprint/environment/WaveParameters` (break `LinearColor` _returnvalue_7) (`.G` (break `LinearColor` _returnvalue_7)) (`.B` (break `LinearColor` _returnvalue_7)) (`.A` (break `LinearColor` _returnvalue_7)))))
        (:`then_7`
          (bind _returnvalue_8 (`KismetMaterialLibrary.GetVectorParameterValue` "/Game/Salvo/Assets/Materials/WaveGen/MPC_WaveParams.MPC_WaveParams" "Set02Wave08"))
          (set `self.Set02Wave08` (make `/Game/Salvo/Blueprint/environment/WaveParameters` (break `LinearColor` _returnvalue_8) (`.G` (break `LinearColor` _returnvalue_8)) (`.B` (break `LinearColor` _returnvalue_8)) (`.A` (break `LinearColor` _returnvalue_8)))))))
    (:`then_1`
      (set `self.WaveSet02` (make `/Game/Salvo/Blueprint/environment/WaveSet` (`self.Set02Wave01`) (`self.Set02Wave02`) (`self.Set02Wave03`) (`self.Set02Wave04`) (`self.Set02Wave05`) (`self.Set02Wave06`) (`self.Set02Wave07`) (`self.Set02Wave08`))))))

(fn `Process Buoyancy`
  (params (Component :type "PrimitiveComponent Object Reference") (`Actor Transform` :type "Transform Structure") (`Point Location` :type "Vector Structure") (Mass :type "Float (double-precision)") (`Test Point Radius` :type "Float (double-precision)") (`Actor Volume` :type "Float (double-precision)") (`Buoyancy Multiplier` :type "Float (double-precision)") (TotalPoints :type Integer) (Time :type "Float (double-precision)"))
  (returns (`Is Under Water` :type Boolean))
  (bind _returnvalue (`KismetMathLibrary.Conv_IntToDouble` TotalPoints))
  (bind _returnvalue_2 (`KismetMathLibrary.TransformLocation` `Actor Transform` `Point Location`))
  (bind (_isunderwater _amount) (`self.Find Wave Height at Point` `Actor Transform` `Point Location` (* Time (`self.Time Multiplier`)) `Test Point Radius`))
  (if _isunderwater
    (`PrimitiveComponent.AddForceAtLocation` Component (/ (* (* (`KismetMathLibrary.MakeVector` 0.0 0.0 (* 980.0 `Buoyancy Multiplier`)) Mass) _amount) _returnvalue) _returnvalue_2 "None")
    (else
      (`PrimitiveComponent.AddForceAtLocation` Component (/ (* (* (`KismetMathLibrary.MakeVector` 0.0 0.0 -980.0) Mass) _amount) _returnvalue) _returnvalue_2 "None")))
  (return _isunderwater))

(fn `UserConstructionScript`
  (`self.Init Global Parameters`)
  (`self.Init Wave Set 1`)
  (`self.Init Wave Set 2`))