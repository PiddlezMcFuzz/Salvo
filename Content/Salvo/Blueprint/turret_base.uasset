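; Base ship turret that binds to its player ship's fire, aim-trace and free-camera events, selected by ShipID.
; Aim traces turn yaw and pitch toward the impact point at constant speed within ship-relative limits, pausing during free camera.
; Projectile path prediction positions the ship's hit marker, scaled by camera distance, and gun pitch is broadcast.
; Firing spawns Shell_Base actors, tracked in an array that prediction ignores until their kill events remove them.
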(event `self.ReceiveBeginPlay`
  (bind _asp_ship_basemovement (castclass `/Game/Salvo/Blueprint/p_ship_basemovement` "/Game/Salvo/Blueprint/p_ship_basemovement.p_ship_basemovement_C"))
  (bind _outactors (`GameplayStatics.GetAllActorsOfClass` _asp_ship_basemovement))
  (bind _asp_ship_basemovement_2 (cast `/Game/Salvo/Blueprint/p_ship_basemovement` (`KismetArrayLibrary.Array_Get` _outactors (`self.ShipID`)))
    (:`then`
      (`|ExecutionSequence`
        (:`then_0`
          (add `/Game/Salvo/Blueprint/p_ship_basemovement.Fire` _asp_ship_basemovement_2 (delegate `Firing`)))
        (:`then_1`
          (add `/Game/Salvo/Blueprint/p_ship_basemovement.AimTrace` _asp_ship_basemovement_2 (delegate `AimTrace`)))
        (:`then_2`
          (add `/Game/Salvo/Blueprint/p_ship_basemovement.FreeCamera` _asp_ship_basemovement_2 (delegate `FreeCamPress`)))))
    (:`CastFailed`
      (`KismetSystemLibrary.PrintString` "Cannot Cast to Player"))))

(event `Firing`
  (bind _shellout (`self.projectile_spawn`))
  (bind _returnvalue (`KismetArrayLibrary.Array_AddUnique` (`self.ShellArray`) _shellout))
  (bind _asshell_base (cast `/Game/Salvo/Blueprint/Shell_Base` _shellout))
  (set `/Game/Salvo/Blueprint/Shell_Base.ShellInt` _returnvalue _asshell_base)
  (add `/Game/Salvo/Blueprint/Shell_Base.Shell_IsKill` _asshell_base (delegate `ShellKill`)))

(event `ShellKill`
  (params (ShellInt :type Integer))
  (bind _shellarray (`self.ShellArray`))
  (`KismetArrayLibrary.Array_RemoveItem` _shellarray (`KismetArrayLibrary.Array_Get` _shellarray ShellInt)))

(event `FreeCamPress`
  (params (`Is Pressed` :type Boolean))
  (bind _shellspawn (`self.ShellSpawn`))
  (if (not `Is Pressed`) :!label _label
    (`|ExecutionSequence`
      (:`then_0`
        (`self.Aiming_yaw` (stale `AimTrace` AimTraceImpactPoint) (`self.turret_attach`) (`self.Traverse Speed`) (`self.TraverseLimit`) (stale `AimTrace` ShipRotateWorld)))
      (:`then_1`
        (bind _gunrotation (`self.aiming_pitch` (stale `AimTrace` AimTraceImpactPoint) (`self.gunattach`) (`self.VerticalAimSpeed`) (`self.Vertical Limit`) (`SceneComponent.K2_GetComponentRotation` (`self.Cylinder`))))))
    (for _array_element (`self.TraceImpactList`)
      (bind (_outhit _outpathpositions _outlasttracedestination _returnvalue) (`GameplayStatics.Blueprint_PredictProjectilePath_ByTraceChannel` (`SceneComponent.K2_GetComponentLocation` _shellspawn) (* (`SceneComponent.GetUpVector` _shellspawn) 5000.0) true 10.0 _array_element false (`self.ShellArray`) "None" 0.0 15.0 10.0))
      (bind _output_get (set `self.GunRotation` _gunrotation))
      (`self.GunPitchEvent` _output_get)
      (bind _hitlocation (`/Game/Salvo/Blueprint/p_ship_basemovement.HitLocation` (stale `self.ReceiveBeginPlay` _asp_ship_basemovement_2)))
      (`SceneComponent.SetVisibility` _hitlocation _returnvalue true)
      (bind (_bblockinghit _binitialoverlap _time _location _impactpoint) (`GameplayStatics.BreakHitResult` _outhit))
      (`SceneComponent.K2_SetWorldLocation` _hitlocation _impactpoint false false)
      (`SceneComponent.SetWorldScale3D` _hitlocation (/ (* (0.001 0.001 0.001) (`KismetMathLibrary.VSize` (- _impactpoint (`SceneComponent.K2_GetComponentLocation` (`/Game/Salvo/Blueprint/p_ship_basemovement.Camera` (stale `self.ReceiveBeginPlay` _asp_ship_basemovement_2)))))) 5.0)))))

(event `AimTrace`
  (params (AimTraceImpactPoint :type "Vector Structure") (ShipRotateWorld :type "Rotator Structure"))
  (goto _label))

(fn `aiming_pitch`
  (params (ImpactIn :type "Vector Structure") (ComponentIn :type "SceneComponent Object Reference") (VerticalSpeed :type "Float (double-precision)") (VerticalLimit :type "Float (double-precision)") (ShipRotateWorld :type "Rotator Structure"))
  (returns (GunRotation :type "Rotator Structure"))
  (bind (_returnvalue_location _returnvalue_rotation) (`KismetMathLibrary.BreakTransform` (`KismetMathLibrary.ConvertTransformToRelative` (`KismetMathLibrary.MakeTransform` (0.0 0.0 0.0) (`KismetMathLibrary.FindLookAtRotation` (`SceneComponent.K2_GetComponentLocation` ComponentIn) ImpactIn)) (`KismetMathLibrary.MakeTransform` (0.0 0.0 0.0) ShipRotateWorld))))
  (bind _returnvalue (`KismetMathLibrary.RInterpTo_Constant` (`SceneComponent.RelativeRotation` ComponentIn) (`KismetMathLibrary.MakeRotator` 0.0 (* (`KismetMathLibrary.ClampAngle` (.pitch _returnvalue_rotation) (* VerticalLimit -1.0) VerticalLimit) -1.0)) (`GameplayStatics.GetWorldDeltaSeconds`) VerticalSpeed))
  (`SceneComponent.K2_SetRelativeRotation` ComponentIn _returnvalue false false)
  (return _returnvalue))

(fn `Aiming_yaw`
  (params (Impact_in :type "Vector Structure") (ComponentIn :type "SceneComponent Object Reference") (TraverseSpeed :type "Float (double-precision)") (TraverseLimit :type "Float (double-precision)") (ShipRotateWorld :type "Rotator Structure"))
  (bind (_returnvalue_location _returnvalue_rotation) (`KismetMathLibrary.BreakTransform` (`KismetMathLibrary.ConvertTransformToRelative` (`KismetMathLibrary.MakeTransform` (0.0 0.0 0.0) (`KismetMathLibrary.FindLookAtRotation` (`SceneComponent.K2_GetComponentLocation` ComponentIn) Impact_in)) (`KismetMathLibrary.MakeTransform` (0.0 0.0 0.0) ShipRotateWorld))))
  (`SceneComponent.K2_SetRelativeRotation` ComponentIn (`KismetMathLibrary.RInterpTo_Constant` (`SceneComponent.RelativeRotation` ComponentIn) (`KismetMathLibrary.MakeRotator` (.roll ShipRotateWorld) (.pitch ShipRotateWorld) (* (`KismetMathLibrary.ClampAngle` (.yaw _returnvalue_rotation) (* TraverseLimit -1.0) TraverseLimit) -1.0)) (`GameplayStatics.GetWorldDeltaSeconds`) TraverseSpeed) false false))

(fn `projectile_spawn`
  (returns (ShellOut :type "Actor Object Reference"))
  (bind _returnvalue (`|SpawnActorFromClass` "/Game/Salvo/Blueprint/Shell_Base.Shell_Base_C" (`KismetMathLibrary.MakeTransform` (`SceneComponent.K2_GetComponentLocation` (`self.ShellSpawn`)) (`KismetMathLibrary.Conv_VectorToRotator` (`SceneComponent.GetUpVector` (`self.gun`)))) "Undefined" "OverrideRootScale"))
  (return _returnvalue))

(fn `UserConstructionScript`)