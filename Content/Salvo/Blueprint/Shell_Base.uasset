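; Base projectile actor for a fired shell in Salvo, driven by physics and destroyed on impact.
; On BeginPlay it applies a forward impulse scaled by Firepower and stores ShellForce as that impulse magnitude divided by mass.
; Hits and overlaps with OceanDepthTest share one path that destroys the actor, calls ShellIsKill and prints the hit component's name for debugging.
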(event `self.ReceiveBeginPlay`
  (bind _returnvalue (* (* (`SceneComponent.GetForwardVector` (`self.ShellBase`)) (`self.Firepower`)) 200.0))
  (`PrimitiveComponent.AddImpulse` (`self.shell`) _returnvalue "None" false)
  (set `self.ShellForce` (`KismetMathLibrary.VSize` (/ _returnvalue (`PrimitiveComponent.GetMass` (`self.shell`))))))

(event `self.ReceiveTick`
  (params (DeltaSeconds :type "Float (single-precision)")))

(event `self.ReceiveHit`
  (params (MyComp :type "PrimitiveComponent Object Reference") (Other :type "Actor Object Reference") (OtherComp :type "PrimitiveComponent Object Reference") (bSelfMoved :type Boolean) (HitLocation :type "Vector Structure") (HitNormal :type "Vector Structure") (NormalImpulse :type "Vector Structure") (Hit :type "HitResult Structure (by ref)"))
  (`self.K2_DestroyActor` :!label _label)
  (`self.Shell_IsKill` 0)
  (`KismetSystemLibrary.PrintString` (`KismetSystemLibrary.GetDisplayName` OtherComp)))

(event `self.ReceiveActorBeginOverlap`
  (params (OtherActor :type "Actor Object Reference"))
  (cast `/Game/Salvo/Blueprint/environment/OceanDepthTest` OtherActor)
  (goto _label))

(event `self.shell.OnComponentHit`
  (params (HitComponent :type "PrimitiveComponent Object Reference") (OtherActor :type "Actor Object Reference") (OtherComp :type "PrimitiveComponent Object Reference") (NormalImpulse :type "Vector Structure") (Hit :type "HitResult Structure (by ref)"))
  (goto _label))

(fn `UserConstructionScript`)