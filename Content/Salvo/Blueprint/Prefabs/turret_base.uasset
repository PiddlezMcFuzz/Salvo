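; Base ship turret that aims, fires and takes damage, driven by events from its parent p_ship_basemovement.
; Aim traces drive clamped yaw and pitch, centring outside the camera arc, while predicted projectile paths place distance-scaled hit markers.
; Firing spawns reload-gated Shell_Base actors, tracked so predictions ignore them.
; Shell hits lower health and darken the dynamic material; the turret is disabled until repair restores health to near full.
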(event `self.ReceiveHit`
  (params (MyComp :type "PrimitiveComponent Object Reference") (Other :type "Actor Object Reference") (OtherComp :type "PrimitiveComponent Object Reference") (bSelfMoved :type Boolean) (HitLocation :type "Vector Structure") (HitNormal :type "Vector Structure") (NormalImpulse :type "Vector Structure") (Hit :type "HitResult Structure (by ref)"))
  ;[1 1 1] Take Damage
  (bind _asshell_base (cast `/Game/Salvo/Blueprint/Prefabs/Shell_Base` Other))
  (set `self.Health%` (- (`self.Health%`) (/ (`PrimitiveComponent.GetMass` (`/Game/Salvo/Blueprint/Prefabs/Shell_Base.shell` _asshell_base)) (* (- 1.0 (`self.Armor%`)) 100.0))))
  (`MaterialInstanceDynamic.SetVectorParameterValue` (`self.TurretMaterialInst`) "Color" (* (`self.MatInstBasecolor`) (`self.Health%`)))
  (`self.K2_DestroyActor` _asshell_base)
  (bind _asp_ship_basemovement (cast `/Game/Salvo/Blueprint/Prefabs/p_ship_basemovement` (`self.GetParentActor` self)))
  (add `/Game/Salvo/Blueprint/Prefabs/p_ship_basemovement.RepairPress` _asp_ship_basemovement (delegate `Repair`)))

(event `Repair`
  (bind _turretmaterialinst (`self.TurretMaterialInst`))
  ;[1 1 1] Repair
  (goto _label :!via `Open`))

(event `self.ReceiveTick`
  (params (DeltaSeconds :type "Float (single-precision)"))
  (bind _turretmaterialinst (`self.TurretMaterialInst`))
  ;[1 1 1] Repair
  (`|ExecutionSequence`
    (:`then_0`
      (`/Engine/EditorBlueprintResources/StandardMacros.Gate` true :!label _label
        (:`Exit`
          (`|ExecutionSequence`
            (:`then_0`
              (set `self.Health%` (`KismetMathLibrary.FInterpTo_Constant` (`self.Health%`) 1.0 DeltaSeconds 0.5)))
            (:`then_1`
              (bind _returnvalue (`MaterialInstanceDynamic.K2_GetVectorParameterValue` _turretmaterialinst "Color"))
              (`MaterialInstanceDynamic.SetVectorParameterValue` _turretmaterialinst "Color" (`KismetMathLibrary.CInterpTo` _returnvalue (`self.MatInstBasecolor`) DeltaSeconds 0.5)))))))
    (:`then_1`
      (set `self.IsDisabled` (not (`KismetMathLibrary.NearlyEqual_FloatFloat` (`self.Health%`) 1.0 0.075))))))

(event `Firing`
  ;[1 1 1] Firing
  (if (not (or (`self.MovingToZero`) (`self.IsDisabled`)))
    (`/Engine/EditorBlueprintResources/StandardMacros.CompareFloat` (`self.ReloadTimeRelative`) (`KismetSystemLibrary.GetGameTimeInSeconds`)
      (:`<`
        (bind _shellout (`self.projectile_spawn` (`self.Shell Size (mm)`) (`self.Firepower`) (`self.Shell Mass`)))
        (bind _returnvalue (`KismetArrayLibrary.Array_AddUnique` (`self.ShellArray`) _shellout))
        (bind _asshell_base (cast `/Game/Salvo/Blueprint/Prefabs/Shell_Base` _shellout))
        (set `/Game/Salvo/Blueprint/Prefabs/Shell_Base.ShellInt` _returnvalue _asshell_base)
        (add `/Game/Salvo/Blueprint/Prefabs/Shell_Base.Shell_IsKill` _asshell_base (delegate `ShellKill`))
        (set `self.ReloadTimeRelative` (+ (`KismetSystemLibrary.GetGameTimeInSeconds`) (`self.ReloadTime`)))))))

(event `self.ReceiveBeginPlay`
  ;[1 1 1] Get Owning Ship
  (bind _asp_ship_basemovement (cast `/Game/Salvo/Blueprint/Prefabs/p_ship_basemovement` (`self.GetParentActor` self))
    (:`then`
      (`|ExecutionSequence`
        (:`then_0`
          ;[1 1 1] Firing
          (add `/Game/Salvo/Blueprint/Prefabs/p_ship_basemovement.Fire` _asp_ship_basemovement (delegate `Firing`)))
        (:`then_1`
          (add `/Game/Salvo/Blueprint/Prefabs/p_ship_basemovement.AimTrace` _asp_ship_basemovement (delegate `AimTrace`)))
        (:`then_2`
          ;[1 1 1] Check Free Cam Press
          (add `/Game/Salvo/Blueprint/Prefabs/p_ship_basemovement.FreeCamera` _asp_ship_basemovement (delegate `FreeCamPress`)))))
    (:`CastFailed`
      (`KismetSystemLibrary.PrintString` "Cannot Cast to Player" true true (struct :`G` 0.66 :`B` 1.0 :`A` 1.0) 15.0))))

(event `ShellKill`
  (params (ShellInt :type Integer))
  (bind _shellarray (`self.ShellArray`))
  ;[1 1 1] Firing
  (`KismetArrayLibrary.Array_RemoveItem` _shellarray (`KismetArrayLibrary.Array_Get` _shellarray ShellInt)))

(event `FreeCamPress`
  (params (`Is Pressed` :type Boolean))
  (bind _isdisabled (`self.IsDisabled`))
  (bind _shellspawn (`self.ShellSpawn`))
  ;[1 1 1] Check Free Cam Press
  (if (not `Is Pressed`) :!label _label_2
    ;[1 1 1] Aiming
    (`|ExecutionSequence`
      (:`then_0`
        (bind _movingtozero (`self.Aiming_yaw` (stale `AimTrace` AimTraceImpactPoint) (`self.turret_attach`) (`self.Traverse Speed`) (`self.TraverseLimit`) (stale `AimTrace` ShipRotateWorld) (stale `self.ReceiveBeginPlay` _asp_ship_basemovement) _isdisabled))
        (set `self.MovingToZero` _movingtozero))
      (:`then_1`
        (bind _gunrotation (`self.aiming_pitch` (stale `AimTrace` AimTraceImpactPoint) (`self.gunattach`) (`self.VerticalAimSpeed`) (`self.Vertical Limit`) (`SceneComponent.K2_GetComponentRotation` (`self.Cylinder`)) (stale `self.ReceiveBeginPlay` _asp_ship_basemovement) (`self.MovingToZero`) _isdisabled))))
    ;;[1 1 1] Hit Trace
    (for _array_element (`self.TraceImpactList`)
      (bind (_outhit _outpathpositions _outlasttracedestination _returnvalue) (`GameplayStatics.Blueprint_PredictProjectilePath_ByTraceChannel` (`SceneComponent.K2_GetComponentLocation` _shellspawn) (* (`SceneComponent.GetUpVector` _shellspawn) (`self.Firepower`)) true (/ (`self.Shell Size (mm)`) 1000.0) _array_element true (`self.ShellArray`) "None" 0.0 15.0 10.0))
      (bind _output_get (set `self.GunRotation` _gunrotation))
      (`self.GunPitchEvent` _output_get)
      (bind _item (`KismetArrayLibrary.Array_Get` (`/Game/Salvo/Blueprint/Prefabs/p_ship_basemovement.HitLocationArray` (stale `self.ReceiveBeginPlay` _asp_ship_basemovement)) (`self.TurretID`)))
      (`SceneComponent.SetVisibility` _item _returnvalue false)
      (bind (_bblockinghit _binitialoverlap _time _location _impactpoint) (`GameplayStatics.BreakHitResult` _outhit))
      (`SceneComponent.K2_SetWorldLocation` _item _impactpoint false false)
      (`SceneComponent.SetWorldScale3D` _item (/ (* (0.001 0.001 0.001) (`KismetMathLibrary.VSize` (- _impactpoint (`SceneComponent.K2_GetComponentLocation` (`/Game/Salvo/Blueprint/Prefabs/p_ship_basemovement.Camera` (stale `self.ReceiveBeginPlay` _asp_ship_basemovement)))))) 5.0)))))

(event `AimTrace`
  (params (AimTraceImpactPoint :type "Vector Structure") (ShipRotateWorld :type "Rotator Structure"))
  (goto _label_2))

(fn `aiming_pitch`
  (params (ImpactIn :type "Vector Structure") (ComponentIn :type "SceneComponent Object Reference") (VerticalSpeed :type "Float (double-precision)") (VerticalLimit :type "Float (double-precision)") (TurretRotation :type "Rotator Structure") (Ship :type "Pawn Object Reference") (MovingToZero :type Boolean) (IsDisabled :type Boolean))
  (returns (GunRotation :type "Rotator Structure"))
  (bind _returnvalue (`GameplayStatics.GetWorldDeltaSeconds`))
  (bind _relativerotation (`SceneComponent.RelativeRotation` ComponentIn))
  (bind (_returnvalue_location _returnvalue_rotation) (`KismetMathLibrary.BreakTransform` (`KismetMathLibrary.ConvertTransformToRelative` (`KismetMathLibrary.MakeTransform` (0.0 0.0 0.0) (`KismetMathLibrary.FindLookAtRotation` (`SceneComponent.K2_GetComponentLocation` ComponentIn) ImpactIn)) (`KismetMathLibrary.MakeTransform` (0.0 0.0 0.0) TurretRotation))))
  (bind _returnvalue_2 (`KismetMathLibrary.RInterpTo_Constant` _relativerotation (`KismetMathLibrary.MakeRotator` 0.0 (* (`KismetMathLibrary.ClampAngle` (.pitch _returnvalue_rotation) (* VerticalLimit -1.0) VerticalLimit) -1.0)) _returnvalue VerticalSpeed))
  (if (not IsDisabled)
    (if MovingToZero
      (`SceneComponent.K2_SetRelativeRotation` ComponentIn (`KismetMathLibrary.RInterpTo_Constant` _relativerotation (struct) _returnvalue VerticalSpeed) false false)
      (else
        (`SceneComponent.K2_SetRelativeRotation` ComponentIn _returnvalue_2 false false)))
    (return _returnvalue_2)))

(fn `Aiming_yaw`
  (params (Impact_in :type "Vector Structure") (ComponentIn :type "SceneComponent Object Reference") (TraverseSpeed :type "Float (double-precision)") (TraverseLimit :type "Float (double-precision)") (ShipRotateWorld :type "Rotator Structure") (Ship :type "Pawn Object Reference") (IsDisabled :type Boolean))
  (returns (MovingToZero :type Boolean))
  (bind _returnvalue (`GameplayStatics.GetWorldDeltaSeconds`))
  (bind _returnvalue_2 (+ TraverseLimit 10.0))
  (bind _relativerotation (`SceneComponent.RelativeRotation` ComponentIn))
  (bind (_returnvalue_location _returnvalue_rotation) (`KismetMathLibrary.BreakTransform` (`KismetMathLibrary.ConvertTransformToRelative` (`KismetMathLibrary.MakeTransform` (0.0 0.0 0.0) (`KismetMathLibrary.FindLookAtRotation` (`SceneComponent.K2_GetComponentLocation` ComponentIn) Impact_in)) (`KismetMathLibrary.MakeTransform` (0.0 0.0 0.0) (`self.K2_GetActorRotation` Ship)))))
  (if (not IsDisabled)
    (bind _asp_ship_basemovement (cast `/Game/Salvo/Blueprint/Prefabs/p_ship_basemovement` Ship))
    (bind _yaw (.yaw (`SceneComponent.RelativeRotation` (`/Game/Salvo/Blueprint/Prefabs/p_ship_basemovement.CameraMaster` _asp_ship_basemovement))))
    (bind _ship_basecube (`/Game/Salvo/Blueprint/Prefabs/p_ship_basemovement.ship_basecube` _asp_ship_basemovement))
    (bind (_returnvalue_location_2 _returnvalue_rotation_2) (`KismetMathLibrary.BreakTransform` (`KismetMathLibrary.ConvertTransformToRelative` (`SceneComponent.GetSocketTransform` _ship_basecube (`SceneComponent.GetAttachSocketName` (`KismetArrayLibrary.Array_Get` (`/Game/Salvo/Blueprint/Prefabs/p_ship_basemovement.Turrets` _asp_ship_basemovement) (`self.TurretID`))) "RTS_World") (`SceneComponent.K2_GetComponentToWorld` _ship_basecube))))
    (bind _yaw_2 (.yaw _returnvalue_rotation_2))
    (if (or (`KismetMathLibrary.InRange_FloatFloat` _yaw (- _yaw_2 _returnvalue_2) _yaw_2) (`KismetMathLibrary.InRange_FloatFloat` _yaw (* _yaw_2 -1.0) (+ (* (`KismetMathLibrary.FTrunc` (* (`KismetMathLibrary.FClamp` (- _yaw_2 1.0) -1.0) -1.0)) _yaw_2) _returnvalue_2)))
      (`SceneComponent.K2_SetRelativeRotation` ComponentIn (`KismetMathLibrary.RInterpTo_Constant` _relativerotation (`KismetMathLibrary.MakeRotator` (.roll _relativerotation) (.pitch _relativerotation) (`KismetMathLibrary.ClampAxis` (* (`KismetMathLibrary.ClampAngle` (- (.yaw _returnvalue_rotation) _yaw_2) (* TraverseLimit -1.0) TraverseLimit) -1.0))) _returnvalue TraverseSpeed) false false)
      (set `self.MovingToZero` false)
      (else
        (`SceneComponent.K2_SetRelativeRotation` ComponentIn (`KismetMathLibrary.RInterpTo_Constant` _relativerotation (struct) _returnvalue TraverseSpeed) false false)
        (set `self.MovingToZero` true)))
    (return (`self.MovingToZero`))))

(fn `projectile_spawn`
  (params (`Shell Size (mm)` :type "Float (double-precision)") (Firepower :type "Float (double-precision)") (`Shell Mass` :type "Float (double-precision)"))
  (returns (ShellOut :type "Actor Object Reference"))
  (bind _returnvalue (`|SpawnActorFromClass` "/Game/Salvo/Blueprint/Prefabs/Shell_Base.Shell_Base_C" (`KismetMathLibrary.MakeTransform` (`SceneComponent.K2_GetComponentLocation` (`self.ShellSpawn`)) (`KismetMathLibrary.MakeRotator` (.roll (`KismetMathLibrary.Conv_VectorToRotator` (`SceneComponent.GetUpVector` (`self.gun`)))) (- (.pitch (`KismetMathLibrary.Conv_VectorToRotator` (`SceneComponent.GetUpVector` (`self.gun`)))) 90.0) (.yaw (`KismetMathLibrary.Conv_VectorToRotator` (`SceneComponent.GetUpVector` (`self.gun`))))) (* (1.0 1.0 1.0) (/ `Shell Size (mm)` 1000.0))) "Undefined" "OverrideRootScale" null Firepower 0 `Shell Mass`))
  (return _returnvalue))

(fn `UserConstructionScript`
  (bind _turretmaterialinst (`self.TurretMaterialInst`))
  (bind _returnvalue (`KismetMaterialLibrary.CreateDynamicMaterialInstance` (`self.Cylinder`) (`self.TurretMaterial`)))
  (set `self.TurretMaterialInst` _returnvalue)
  (`PrimitiveComponent.SetMaterial` (`self.Cylinder`) 0 _turretmaterialinst)
  (`PrimitiveComponent.SetMaterial` (`self.gun`) 0 _turretmaterialinst)
  (`PrimitiveComponent.SetMaterial` (`self.mantlet`) 0 _turretmaterialinst)
  (bind _returnvalue_2 (`MaterialInstanceDynamic.K2_GetVectorParameterValue` _turretmaterialinst "Color"))
  (set `self.MatInstBasecolor` _returnvalue_2))