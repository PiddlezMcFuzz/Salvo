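; Shell_Base is a physics-driven projectile shell in Salvo that launches itself on spawn and destroys itself on impact.
; BeginPlay overrides the Shell component's mass, then applies a velocity-change impulse along its up vector scaled by Firepower.
; On hit, it waits briefly if the other component has physics collision, then fires the ShellIsKill and ComponentImpact dispatchers, prints the component's name and destroys itself.
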(event `self.ReceiveBeginPlay`
  (bind _shell (`self.shell`))
  (`PrimitiveComponent.SetMassOverrideInKg` _shell "None" (`self.ShellMass`) true)
  (`PrimitiveComponent.AddImpulse` (`self.shell`) (* (`SceneComponent.GetUpVector` _shell) (`self.Firepower`)) "None" true))

(event `self.ReceiveTick`
  (params (DeltaSeconds :type "Float (single-precision)")))

(event `self.ReceiveHit`
  (params (MyComp :type "PrimitiveComponent Object Reference") (Other :type "Actor Object Reference") (OtherComp :type "PrimitiveComponent Object Reference") (bSelfMoved :type Boolean) (HitLocation :type "Vector Structure") (HitNormal :type "Vector Structure") (NormalImpulse :type "Vector Structure") (Hit :type "HitResult Structure (by ref)"))
  (if (`PrimitiveComponent.K2_IsPhysicsCollisionEnabled` OtherComp)
    (`KismetSystemLibrary.Delay` 0.01))
  (`self.Shell_IsKill` (`self.ShellInt`))
  (`self.Component_Impact` OtherComp)
  (`KismetSystemLibrary.PrintString` (`KismetSystemLibrary.GetDisplayName` OtherComp))
  (`self.K2_DestroyActor`))

(fn `UserConstructionScript`)