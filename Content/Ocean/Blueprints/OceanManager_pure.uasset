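; Ocean manager that computes Gerstner wave displacement at a world location on demand from its wavelength, amplitude and direction.
; GetWaveHeightAtLocation averages two clusters at game time, the second smaller, angled differently and phase-shifted, returning a vector despite its name.
; Each cluster averages eight CalculateGerstnerWave calls with varied scale, angle and phase.
; Each wave uses cosine for X but sine for Y and Z, and time is unscaled by wavelength.
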(fn `CalculateGerstnerWave`
  (params (Wavelength :type "Float (double-precision)" :default 0.0) (Amplitude :type "Float (double-precision)" :default 0.0) (Location :type "Vector2D Structure") (Direction :type "Vector2D Structure") (Angle :type "Float (double-precision)" :default 0.0) (Steepness :type "Float (double-precision)" :default 0.5) (Time :type "Float (double-precision)" :default 0.0) (Phase :type "Float (double-precision)" :default 0.0))
  (returns (Delta :type "Vector Structure"))
  (bind (_x _y) (`KismetMathLibrary.BreakVector2D` Direction))
  (bind _returnvalue (* Steepness Amplitude))
  (bind _returnvalue_2 (`KismetMathLibrary.Normal2D` (`KismetMathLibrary.Conv_VectorToVector2D` (`KismetMathLibrary.RotateAngleAxis` (`KismetMathLibrary.MakeVector` _x _y) (* Angle 360.0) (0.0 0.0 1.0)))))
  (bind (_x_2 _y_2) (`KismetMathLibrary.BreakVector2D` _returnvalue_2))
  (bind _returnvalue_3 (+ (* (/ (`KismetMathLibrary.MultiplyByPi` 2.0) Wavelength) (`KismetMathLibrary.DotProduct2D` Location _returnvalue_2)) Time Phase))
  (bind _returnvalue_4 (`KismetMathLibrary.Sin` _returnvalue_3))
  (return (`KismetMathLibrary.MakeVector` (* _returnvalue _x_2 (`KismetMathLibrary.Cos` _returnvalue_3)) (* _returnvalue _y_2 _returnvalue_4) (* _returnvalue_4 Amplitude))))

(fn `CalculateGerstnerWaveCluster`
  (params (MedianWavelength :type "Float (double-precision)" :default 0.0) (MedianAmplitude :type "Float (double-precision)" :default 0.0) (Location :type "Vector2D Structure") (MedianDirection :type "Vector2D Structure") (MedianAngle :type "Float (double-precision)" :default 0.0) (Steepness :type "Float (double-precision)" :default 0.0) (Time :type "Float (double-precision)" :default 0.0) (MedianPhase :type "Float (double-precision)" :default 0.0))
  (returns (Delta :type "Vector Structure"))
  (locals (Sum :type "Vector Structure"))
  (bind _sum (`local.Sum`))
  (`|ExecutionSequence`
    (:`then_0`
      (bind _delta (`self.CalculateGerstnerWave` MedianWavelength MedianAmplitude Location MedianDirection MedianAngle Steepness Time MedianPhase))
      (set `local.Sum` (+ _sum _delta)))
    (:`then_1`
      (bind _delta_2 (`self.CalculateGerstnerWave` (* MedianWavelength 0.5) (* MedianAmplitude 0.5) Location MedianDirection (+ MedianAngle -0.058) Steepness Time (+ MedianPhase 1.0)))
      (set `local.Sum` (+ _sum _delta_2)))
    (:`then_2`
      (bind _delta_3 (`self.CalculateGerstnerWave` (* MedianWavelength 2.0) (* MedianAmplitude 2.0) Location MedianDirection (+ MedianAngle -0.047) Steepness Time (+ MedianPhase -1.5)))
      (set `local.Sum` (+ _sum _delta_3)))
    (:`then_3`
      (bind _delta_4 (`self.CalculateGerstnerWave` (* MedianWavelength 1.25) (* MedianAmplitude 1.25) Location MedianDirection (+ MedianAngle 0.05) Steepness Time (+ MedianPhase 0.75)))
      (set `local.Sum` (+ _sum _delta_4)))
    (:`then_4`
      (bind _delta_5 (`self.CalculateGerstnerWave` (* MedianWavelength 0.75) (* MedianAmplitude 0.75) Location MedianDirection (+ MedianAngle 0.075) Steepness Time (+ MedianPhase -0.6)))
      (set `local.Sum` (+ _sum _delta_5)))
    (:`then_5`
      (bind _delta_6 (`self.CalculateGerstnerWave` (* MedianWavelength 1.5) (* MedianAmplitude 1.5) Location MedianDirection (+ MedianAngle -0.083) Steepness Time (+ MedianPhase 0.9)))
      (set `local.Sum` (+ _sum _delta_6)))
    (:`then_6`
      (bind _delta_7 (`self.CalculateGerstnerWave` (* MedianWavelength 0.825) (* MedianAmplitude 0.825) Location MedianDirection (+ MedianAngle 0.063) Steepness Time (+ MedianPhase -0.23)))
      (set `local.Sum` (+ _sum _delta_7)))
    (:`then_7`
      (bind _delta_8 (`self.CalculateGerstnerWave` (* MedianWavelength 0.65) (* MedianAmplitude 0.65) Location MedianDirection (+ MedianAngle -0.011) Steepness Time (+ MedianPhase 1.72)))
      (set `local.Sum` (+ _sum _delta_8)))
    (:`then_8`
      (return (/ (`local.Sum`) 8.0)))))

(fn `GetWaveHeightAtLocation`
  (params (Location :type "Vector Structure" :default (0.0 0.0 0.0)))
  (returns (Delta :type "Vector Structure"))
  (bind _returnvalue (`KismetSystemLibrary.GetGameTimeInSeconds`))
  (bind _wavelength (`self.Wavelength`))
  (bind _amplitude (`self.Amplitude`))
  (bind _direction (`self.Direction`))
  (bind _delta (`self.CalculateGerstnerWaveCluster` _wavelength _amplitude (`KismetMathLibrary.Conv_VectorToVector2D` Location) _direction -0.015 0.5 _returnvalue))
  (bind _delta_2 (`self.CalculateGerstnerWaveCluster` (* _wavelength 0.6) (* _amplitude 0.6) (`KismetMathLibrary.Conv_VectorToVector2D` Location) _direction 0.015 0.5 _returnvalue 1.2))
  (return (/ (+ _delta _delta_2) 2.0)))

(fn `UserConstructionScript`)