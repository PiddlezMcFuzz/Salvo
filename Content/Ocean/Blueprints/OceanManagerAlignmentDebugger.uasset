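; OceanManagerAlignmentDebugger is a debug Blueprint, apparently for checking alignment with the OceanManager's wave heights.
; Its construction script fills TestPoints with a flat local-space grid centered on the actor, sized by GridCount and Size.
; Each Tick transforms the points to world space, queries GetWaveHeightAtLocation for each, and draws a red debug sphere from the transformed position.
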(event `self.ReceiveTick`
  (params (DeltaSeconds :type "Float (single-precision)"))
  (for _array_element (`self.TestPoints`)
    (bind _returnvalue (`KismetMathLibrary.TransformLocation` (`self.GetTransform`) _array_element))
    (`/Game/Ocean/Blueprints/OceanManager.GetWaveHeightAtLocation` (`self.OceanManager`) _returnvalue)
    (`KismetSystemLibrary.DrawDebugSphere` (+ _returnvalue (`KismetMathLibrary.MakeVector` (.x _returnvalue) (.y _returnvalue) (+ (.z _returnvalue) (.z (0.0 0.0 0.0))))) 50.0 5 (struct :`R` 1.0 :`A` 1.0) -1.0)))

(fn `UserConstructionScript`
  (bind _size (`self.Size`))
  (bind _returnvalue (/ (`self.Grid Count`) 2))
  (bind _returnvalue_2 (- 0 _returnvalue))
  (for _index (range _returnvalue_2 (+ _returnvalue 1))
    (for _index_2 (range _returnvalue_2 (+ _returnvalue 1))
      (`KismetArrayLibrary.Array_Add` (`self.TestPoints`) (`KismetMathLibrary.MakeVector` (* _index _size) (* _index_2 _size))))))